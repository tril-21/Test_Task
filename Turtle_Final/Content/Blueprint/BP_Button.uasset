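; BP_Button is an interactable button that shows a hint when the player character approaches and triggers a linked spawner.
; Its Box overlap stores the button on BP_Character and clears that reference on exit, calling BP_GameMode's ShowWidget in both cases.
; Event_Spawn, which nothing in this graph calls, forwards to FuncSpawnMessage on the referenced ActorSpawn.
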(event OnComponentBeginOverlap(Box)
  (params (OverlappedComponent :type Primitive%20Component%20Object%20Reference) (OtherActor :type Actor%20Object%20Reference) (OtherComp :type Primitive%20Component%20Object%20Reference) (OtherBodyIndex :type Integer) (bFromSweep :type Boolean) (SweepResult :type Hit%20Result%20Structure%20%28by%20ref%29))
  ;[1 1 1] Запуск подсказки. Запоминание кнопки, к которой подошли
  (bind _asbp_character (Utilities|Casting|CastToBP_Character OtherActor))
  (Variables|/Game/Blueprint/BP_Character.BP_Character_C|SetButton _asbp_character self)
  (Default|ShowWidget (.AsBP%20Game%20Mode (Utilities|Casting|CastToBP_GameMode (Game|GetGameMode)))))

(event OnComponentEndOverlap(Box)
  (params (OverlappedComponent :type Primitive%20Component%20Object%20Reference) (OtherActor :type Actor%20Object%20Reference) (OtherComp :type Primitive%20Component%20Object%20Reference) (OtherBodyIndex :type Integer))
  ;[1 1 1] Запуск подсказки. Запоминание кнопки, к которой подошли
  (bind _asbp_character (Utilities|Casting|CastToBP_Character OtherActor))
  (Variables|/Game/Blueprint/BP_Character.BP_Character_C|SetButton _asbp_character 0)
  (Default|ShowWidget (.AsBP%20Game%20Mode (Utilities|Casting|CastToBP_GameMode (Game|GetGameMode)))))

(event Custom|Event_Spawn
  (Class|BPIActSpawn|FuncSpawn(Message) (Variables|Default|GetActor_Spawn)))

(event EventBeginPlay)

(event Collision|EventActorBeginOverlap
  (params (OtherActor :type Actor%20Object%20Reference)))

(event EventTick
  (params (DeltaSeconds :type Float%20%28single-precision%29)))

(fn ConstructionScript)