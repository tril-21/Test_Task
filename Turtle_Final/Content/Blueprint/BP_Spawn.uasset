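; BP_Spawn is a spawn point actor that creates BP_Character_NPC instances at its own location.
; FuncSpawn first triggers Player_Effects, which plays a 2D collapse sound and spawns an explosion emitter at the spawner.
; It then spawns the NPC, hands it the ActorTarget location, the spawn location and Number, and calls CopyTarget on it.
; Nothing in this Blueprint calls FuncSpawn, and its BeginPlay and Tick are unused.
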(event Custom|Player_Effects
  (Audio|PlaySound2D "/Game/StarterContent/Audio/Collapse_Cue.Collapse_Cue" 1.0 1.0 0.0 0 0)
  (Effects|SpawnEmitteratLocation "/Game/StarterContent/Particles/P_Explosion.P_Explosion" (Transformation|GetActorLocation self)))

(event EventBeginPlay)

(event Collision|EventActorBeginOverlap
  (params (OtherActor :type Actor%20Object%20Reference)))

(event EventTick
  (params (DeltaSeconds :type Float%20%28single-precision%29)))

(fn ConstructionScript)

(fn FuncSpawn
  (CallFunction|PlayerEffects)
  (bind _returnvalue (Game|SpawnActorfromClass "/Game/Blueprint/BP_Character_NPC.BP_Character_NPC_C" (Math|Transform|MakeTransform (Transformation|GetActorLocation)) "Undefined" 0 0))
  (Variables|/Game/Blueprint/BP_Character_NPC.BP_Character_NPC_C|SetTarget_Location _returnvalue (Transformation|GetActorLocation (Variables|Default|GetActor_Target)))
  (Variables|/Game/Blueprint/BP_Character_NPC.BP_Character_NPC_C|SetStart_Target_Location _returnvalue (Transformation|GetActorLocation self))
  (Variables|/Game/Blueprint/BP_Character_NPC.BP_Character_NPC_C|SetNumber _returnvalue (Variables|Default|Getnumber))
  (Default|CopyTarget _returnvalue))